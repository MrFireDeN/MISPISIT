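; Main player character Blueprint that handles view switching and interaction with objects.
; The V key calls ChangeView, which is defined outside these graphs, and Tick calls HandleCameraTransition.
; Actor overlaps and the DetachInteractable event forward to BPIntaractComponent for touch, untouch and detach.
; HandleCameraTransition and ToggleCamera have empty bodies, leaving their TInterpTo camera-blend and swap logic disconnected, along with a yaw-rotation toggle.
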(event Custom|DetachInteractable
  (Default|Detach (Variables|Default|GetBP_IntaractComponent)))

(event EventBeginPlay)

(event Collision|EventActorBeginOverlap
  (params (OtherActor :type Actor%20Object%20Reference))
  (Default|OnTouch (Variables|Default|GetBP_IntaractComponent) OtherActor))

(event Collision|EventActorEndOverlap
  (params (OtherActor :type Actor%20Object%20Reference))
  (Default|OnUntouch (Variables|Default|GetBP_IntaractComponent) OtherActor))

(event EventTick
  (params (DeltaSeconds :type Float%20%28single-precision%29))
  (CallFunction|HandleCameraTransition DeltaSeconds))

(event Input|KeyboardEvents|V
  (params (Key :type Key%20Structure :default "None"))
  (:Pressed
    (Class|MIPlayerCharacter|ChangeView)))

(fn ConstructionScript)

(fn ToggleCamera
  (params (NewCamera :type Camera%20Component%20Object%20Reference)))

(fn HandleCameraTransition
  (params (DeltaTime :type Float%20%28single-precision%29)))