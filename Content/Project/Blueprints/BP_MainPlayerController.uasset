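; Player controller that turns input into movement, camera and interaction actions for BP_MainCharacter.
; On BeginPlay it adds the Enhanced Input mapping context and caches the character, then handles camera-relative movement, jump, hold-to-sprint, look and view switching.
; Interact has the character's BPIntaractComponent attach to the right-hand socket.
; Raw mouse buttons and number keys 1–6 are forwarded to that component's attached actor as generic primary, secondary and numeric actions.
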(event Input|EnhancedActionEvents|EnhancedInputActionIA_Move
  (params (ActionValue :type Vector%202D%20Structure) (ElapsedSeconds :type Float%20%28double-precision%29) (TriggeredSeconds :type Float%20%28double-precision%29) (InputAction :type Input%20Action%20Object%20Reference :default "/Game/Project/Input/Actions/IA_Move.IA_Move"))
  (bind _returnvalue (Game|GetPlayerCameraManager 0))
  (bind (_x _y) (Math|Vector2D|BreakVector2D ActionValue))
  (bind _rootcomponent (Variables|/Script/Engine.Actor|GetRootComponent _returnvalue))
  (bind _returnvalue_2 (Math|Vector|GetForwardVector _rootcomponent))
  ;[1 0 0 0.5] Movement
  (:Triggered
    (Pawn|Input|AddMovementInput (Variables|Default|GetAs%20Character) (+ (* (Math|Vector|Normalize (Math|Vector|MakeVector (.x _returnvalue_2) (.y _returnvalue_2) 0.0)) _y) (* (Math|Vector|GetRightVector _rootcomponent) _x)) 1.0 false)))

(event Input|EnhancedActionEvents|EnhancedInputActionIA_Look
  (params (ActionValue :type Vector%202D%20Structure) (ElapsedSeconds :type Float%20%28double-precision%29) (TriggeredSeconds :type Float%20%28double-precision%29) (InputAction :type Input%20Action%20Object%20Reference :default "/Game/Project/Input/Actions/IA_Look.IA_Look"))
  (bind (_x _y) (Math|Vector2D|BreakVector2D ActionValue))
  (bind _as_character (Variables|Default|GetAs%20Character))
  ;[0 0.5 1] Camera
  (:Triggered
    (Pawn|Input|AddControllerYawInput _as_character _x)
    (Pawn|Input|AddControllerPitchInput _as_character _y)))

(event Input|EnhancedActionEvents|EnhancedInputActionIA_ChangeView
  (params (ActionValue :type Boolean) (ElapsedSeconds :type Float%20%28double-precision%29) (TriggeredSeconds :type Float%20%28double-precision%29) (InputAction :type Input%20Action%20Object%20Reference :default "/Game/Project/Input/Actions/IA_ChangeView.IA_ChangeView"))
  (bind _as_bp_main_character (Variables|Default|GetAs%20BP%20Main%20Character))
  ;[0 0.5 1] Camera
  (:Started
    (Utilities|IsValid _as_bp_main_character
      (:Is%20Valid
        (Default|ChangeView _as_bp_main_character)))))

(event Input|EnhancedActionEvents|EnhancedInputActionIA_Jump
  (params (ActionValue :type Boolean) (ElapsedSeconds :type Float%20%28double-precision%29) (TriggeredSeconds :type Float%20%28double-precision%29) (InputAction :type Input%20Action%20Object%20Reference :default "/Game/Project/Input/Actions/IA_Jump.IA_Jump"))
  (bind _as_character (Variables|Default|GetAs%20Character))
  ;[1 0 0 0.5] Movement
  (:Triggered
    (Character|Jump _as_character))
  (:Canceled
    (Character|StopJumping _as_character)))

(event Input|EnhancedActionEvents|EnhancedInputActionIA_Sprint
  (params (ActionValue :type Boolean) (ElapsedSeconds :type Float%20%28double-precision%29) (TriggeredSeconds :type Float%20%28double-precision%29) (InputAction :type Input%20Action%20Object%20Reference :default "/Game/Project/Input/Actions/IA_Sprint.IA_Sprint"))
  (bind _as_character (Variables|Default|GetAs%20Character))
  (bind _charactermovement (Variables|/Script/Engine.Character|GetCharacterMovement _as_character))
  ;[1 0 0 0.5] Movement
  (:Started
    (Variables|/Script/Engine.CharacterMovementComponent|SetMaxWalkSpeed _charactermovement 1.2e+03))
  (:Canceled
    (Variables|/Script/Engine.CharacterMovementComponent|SetMaxWalkSpeed _charactermovement 6e+02 :!label _label))
  (:Completed
    (goto _label)))

(event Input|EnhancedActionEvents|EnhancedInputActionIA_Interact
  (params (ActionValue :type Boolean) (ElapsedSeconds :type Float%20%28double-precision%29) (TriggeredSeconds :type Float%20%28double-precision%29) (InputAction :type Input%20Action%20Object%20Reference :default "/Game/Project/Input/Actions/IA_Interact.IA_Interact"))
  (bind _as_bp_main_character (Variables|Default|GetAs%20BP%20Main%20Character))
  ;[0.2526 1 0.245] Interaction
  (:Started
    (Utilities|IsValid _as_bp_main_character
      (:Is%20Valid
        (Default|Attach (Variables|/Game/Project/Blueprints/BP_MainCharacter.BP_MainCharacter_C|GetBP_IntaractComponent _as_bp_main_character) "rightHand" (Variables|/Script/Engine.Character|GetMesh _as_bp_main_character))))))

(event EventBeginPlay
  (Variables|Default|SetAs%20Character (Game|GetPlayerCharacter 0))
  (Input|AddMappingContext (PlayerController|LocalPlayerSubsystems|GetEnhancedInputLocalPlayerSubsystem) "/Game/Project/Input/IMC_Default.IMC_Default" 0 "(bIgnoreAllPressedKeysUntilRelease=True,bForceImmediately=False)")
  (bind _asbp_main_character (Utilities|Casting|CastToBP_MainCharacter (Variables|Default|GetAs%20Character)))
  (Variables|Default|SetAs%20BP%20Main%20Character _asbp_main_character))

(event EventTick
  (params (DeltaSeconds :type Float%20%28single-precision%29)))

(event Input|KeyboardEvents|6
  (params (Key :type Key%20Structure :default "None"))
  (bind _as_bp_main_character (Variables|Default|GetAs%20BP%20Main%20Character))
  ;[1 0.5428 0] Interactable Input
  (:Pressed
    (Utilities|IsValid _as_bp_main_character
      (:Is%20Valid
        (Class|InteractableHelper|CallonNumericAction (Variables|/Game/Project/Blueprints/BP_InteractComponent.BP_InteractComponent_C|GetAttachedActor (Variables|/Game/Project/Blueprints/BP_MainCharacter.BP_MainCharacter_C|GetBP_IntaractComponent _as_bp_main_character)) 6)))))

(event Input|MouseEvents|RightMouseButton
  (params (Key :type Key%20Structure :default "None"))
  (bind _as_bp_main_character (Variables|Default|GetAs%20BP%20Main%20Character))
  ;[1 0.5428 0] Interactable Input
  (:Pressed
    (Utilities|IsValid _as_bp_main_character
      (:Is%20Valid
        (Class|InteractableHelper|CallonSecondaryAction (Variables|/Game/Project/Blueprints/BP_InteractComponent.BP_InteractComponent_C|GetAttachedActor (Variables|/Game/Project/Blueprints/BP_MainCharacter.BP_MainCharacter_C|GetBP_IntaractComponent _as_bp_main_character)))))))

(event Input|KeyboardEvents|2
  (params (Key :type Key%20Structure :default "None"))
  (bind _as_bp_main_character (Variables|Default|GetAs%20BP%20Main%20Character))
  ;[1 0.5428 0] Interactable Input
  (:Pressed
    (Utilities|IsValid _as_bp_main_character
      (:Is%20Valid
        (Class|InteractableHelper|CallonNumericAction (Variables|/Game/Project/Blueprints/BP_InteractComponent.BP_InteractComponent_C|GetAttachedActor (Variables|/Game/Project/Blueprints/BP_MainCharacter.BP_MainCharacter_C|GetBP_IntaractComponent _as_bp_main_character)) 2)))))

(event Input|KeyboardEvents|3
  (params (Key :type Key%20Structure :default "None"))
  (bind _as_bp_main_character (Variables|Default|GetAs%20BP%20Main%20Character))
  ;[1 0.5428 0] Interactable Input
  (:Pressed
    (Utilities|IsValid _as_bp_main_character
      (:Is%20Valid
        (Class|InteractableHelper|CallonNumericAction (Variables|/Game/Project/Blueprints/BP_InteractComponent.BP_InteractComponent_C|GetAttachedActor (Variables|/Game/Project/Blueprints/BP_MainCharacter.BP_MainCharacter_C|GetBP_IntaractComponent _as_bp_main_character)) 3)))))

(event Input|KeyboardEvents|4
  (params (Key :type Key%20Structure :default "None"))
  (bind _as_bp_main_character (Variables|Default|GetAs%20BP%20Main%20Character))
  ;[1 0.5428 0] Interactable Input
  (:Pressed
    (Utilities|IsValid _as_bp_main_character
      (:Is%20Valid
        (Class|InteractableHelper|CallonNumericAction (Variables|/Game/Project/Blueprints/BP_InteractComponent.BP_InteractComponent_C|GetAttachedActor (Variables|/Game/Project/Blueprints/BP_MainCharacter.BP_MainCharacter_C|GetBP_IntaractComponent _as_bp_main_character)) 4)))))

(event Input|KeyboardEvents|5
  (params (Key :type Key%20Structure :default "None"))
  (bind _as_bp_main_character (Variables|Default|GetAs%20BP%20Main%20Character))
  ;[1 0.5428 0] Interactable Input
  (:Pressed
    (Utilities|IsValid _as_bp_main_character
      (:Is%20Valid
        (Class|InteractableHelper|CallonNumericAction (Variables|/Game/Project/Blueprints/BP_InteractComponent.BP_InteractComponent_C|GetAttachedActor (Variables|/Game/Project/Blueprints/BP_MainCharacter.BP_MainCharacter_C|GetBP_IntaractComponent _as_bp_main_character)) 5)))))

(event Input|KeyboardEvents|1
  (params (Key :type Key%20Structure :default "None"))
  (bind _as_bp_main_character (Variables|Default|GetAs%20BP%20Main%20Character))
  ;[1 0.5428 0] Interactable Input
  (:Pressed
    (Utilities|IsValid _as_bp_main_character
      (:Is%20Valid
        (Class|InteractableHelper|CallonNumericAction (Variables|/Game/Project/Blueprints/BP_InteractComponent.BP_InteractComponent_C|GetAttachedActor (Variables|/Game/Project/Blueprints/BP_MainCharacter.BP_MainCharacter_C|GetBP_IntaractComponent _as_bp_main_character)) 1)))))

(event Input|MouseEvents|LeftMouseButton
  (params (Key :type Key%20Structure :default "None"))
  (bind _as_bp_main_character (Variables|Default|GetAs%20BP%20Main%20Character))
  ;[1 0.5428 0] Interactable Input
  (:Pressed
    (Utilities|IsValid _as_bp_main_character
      (:Is%20Valid
        (Class|InteractableHelper|CallonPrimaryAction (Variables|/Game/Project/Blueprints/BP_InteractComponent.BP_InteractComponent_C|GetAttachedActor (Variables|/Game/Project/Blueprints/BP_MainCharacter.BP_MainCharacter_C|GetBP_IntaractComponent _as_bp_main_character)))))))

(fn ConstructionScript)