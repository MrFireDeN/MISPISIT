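; BP_GameState is a game state Blueprint that builds, tears down and rebuilds a simple house at a fixed location.
; CreateHouse asks a BuildingFactory, if valid, for a door, a window-type wall, a window and a roof, storing each reference.
; DestroyHouse safely destroys and clears those references, and UpdateHouse chains destroy then create to regenerate the house.
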(event Custom|CreateHouse
  (bind _buildingfactory (Variables|Default|GetBuildingFactory))
  (Utilities|IsValid _buildingfactory
    (:Is%20Valid
      (bind _returnvalue (Class|CPPBuildingFactory|CreateDoor _buildingfactory (Math|Transform|MakeTransform "1200.000000,1200.000000,0.000000" "0.000000,90.000000,0.000000" "1.000000,1.000000,1.000000")))
      (Variables|Default|SetDoor _returnvalue)
      (bind _returnvalue_2 (Class|CPPBuildingFactory|CreateWall _buildingfactory (Math|Transform|MakeTransform "1200.000000,1300.000000,0.000000" "0.000000,90.000000,0.000000" "1.000000,1.000000,1.000000") "ForWindow"))
      (Variables|Default|SetWall _returnvalue_2)
      (bind _returnvalue_3 (Class|CPPBuildingFactory|CreateWindow _buildingfactory (Math|Transform|MakeTransform "1200.000000,1300.000000,0.000000" "0.000000,90.000000,0.000000" "1.000000,1.000000,1.000000")))
      (Variables|Default|SetWindow _returnvalue_3)
      (bind _returnvalue_4 (Class|CPPBuildingFactory|CreateRoof _buildingfactory (Math|Transform|MakeTransform "1200.000000,1200.000000,300.000000" "0.000000,90.000000,0.000000" "2.000000,1.000000,1.000000")))
      (Variables|Default|SetRoof _returnvalue_4))))

(event Custom|DestroyHouse
  (CallFunction|SaveDestoryBuilding (Variables|Default|GetDoor))
  (CallFunction|SaveDestoryBuilding (Variables|Default|GetRoof))
  (CallFunction|SaveDestoryBuilding (Variables|Default|GetWall))
  (CallFunction|SaveDestoryBuilding (Variables|Default|GetWindow))
  (Variables|Default|SetDoor 0)
  (Variables|Default|SetRoof 0)
  (Variables|Default|SetWall 0)
  (Variables|Default|SetWindow 0))

(event Custom|UpdateHouse
  (CallFunction|DestroyHouse)
  (CallFunction|CreateHouse))

(event Custom|SaveDestoryBuilding
  (params (BuildingComponent :type CPP%20Building%20Component%20Object%20Reference))
  (Utilities|IsValid BuildingComponent
    (:Is%20Valid
      (Actor|DestroyActor BuildingComponent))))

(event EventBeginPlay)

(event EventTick
  (params (DeltaSeconds :type Float%20%28single-precision%29)))

(fn ConstructionScript)