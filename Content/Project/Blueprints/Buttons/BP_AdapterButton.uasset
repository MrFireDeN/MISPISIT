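; BP_AdapterButton is a pressable button Blueprint that exercises a C++ gas adapter on a gas cylinder and prints the results.
; On BeginPlay it constructs a CPP_GasAdapter and initializes it with the GasCylinder reference.
; Each press prints the current data and a pressure change calculated from T0 and DT, then applies mass and volume changes and prints the updated data.
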(event EventBeginPlay
  (|CallParentFunction)
  (bind _returnvalue (Game|ConstructObjectfromClass "/Script/MISPISIT.CPP_GasAdapter"))
  (bind _output_get (Variables|Default|SetGasAdapter _returnvalue))
  (Class|CPPGasAdapter|Initialize _output_get (Variables|Default|GetGasCylinder)))

(event EventPress
  (|CallParentFunction)
  ;[1 1 1] Get Data
  (Development|PrintString "OLD DATA:")
  (Development|PrintString (Class|CPPGasAdapter|GetData (Variables|Default|GetGasAdapter)))
  ;[1 1 1] Calculate Dp
  (bind _returnvalue (Class|CPPGasAdapter|CalculateDp (Variables|Default|GetGasAdapter) (Variables|Default|GetT0) (Variables|Default|GetdT)))
  (Development|PrintText (Utilities|Text|FormatText "Calculate DP: {Temp}" _returnvalue))
  ;[1 1 1] Modif Mass
  (Class|CPPGasAdapter|ModifMass (Variables|Default|GetGasAdapter) (Variables|Default|GetdMass))
  ;[1 1 1] ModifVolume
  (Class|CPPGasAdapter|ModifVolume (Variables|Default|GetGasAdapter) (Variables|Default|GetdVolume))
  ;[1 1 1] Get Data
  (Development|PrintString "NEW DATA:")
  (Development|PrintString (Class|CPPGasAdapter|GetData (Variables|Default|GetGasAdapter))))

(fn ConstructionScript
  (|CallParentFunction))