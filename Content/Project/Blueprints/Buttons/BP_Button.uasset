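; Pressure button actor that sinks while any actor overlaps it and rises once all have left.
; Begin and end overlap maintain a list of occupants, calling Press for the first to arrive and Unpress when the list empties.
; Press and Unpress only set a target height, which Tick eases the button mesh's relative Z toward with FInterpTo until nearly equal.
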(event Custom|Press
  (Variables|Default|SetTargetHeight -8.0))

(event Custom|Unpress
  (Variables|Default|SetTargetHeight 0.0))

(event EventBeginPlay
  (Variables|Default|SetTargetHeight 0.0))

(event Collision|EventActorBeginOverlap
  (params (OtherActor :type Actor%20Object%20Reference))
  (Utilities|FlowControl|Sequence
    (:then_0
      (if (Utilities|Array|IsEmpty (Variables|Default|GetOverlapActors))
        (CallFunction|Press)))
    (:then_1
      (Utilities|Array|AddUnique (Variables|Default|GetOverlapActors) OtherActor))))

(event EventTick
  (params (DeltaSeconds :type Float%20%28single-precision%29))
  (CallFunction|SetCurrentButtonZ DeltaSeconds))

(event Collision|EventActorEndOverlap
  (params (OtherActor :type Actor%20Object%20Reference))
  (Utilities|Array|RemoveItem (Variables|Default|GetOverlapActors) OtherActor)
  (if (Utilities|Array|IsEmpty (Variables|Default|GetOverlapActors))
    (CallFunction|Unpress)))

(fn ConstructionScript)

(fn SetCurrentButtonZ
  (params (DeltaTime :type Float%20%28double-precision%29))
  (bind _buttonmesh (Variables|Default|GetButtonMesh))
  (bind _buttonmesh_2 (Variables|Default|GetButtonMesh))
  (bind _relativelocation (Variables|/Script/Engine.SceneComponent|GetRelativeLocation _buttonmesh_2))
  (bind _relativelocation_2 (Variables|/Script/Engine.SceneComponent|GetRelativeLocation _buttonmesh))
  (if (not (Math|Float|NearlyEqual(Float) (Variables|Default|GetTargetHeight) (.z _relativelocation_2) 0.1))
    (Transformation|SetRelativeLocation (Variables|Default|GetButtonMesh) (Math|Vector|MakeVector (.x _relativelocation) (.y _relativelocation) (Math|Interpolation|FInterpTo (.z _relativelocation_2) (Variables|Default|GetTargetHeight) DeltaTime 16.0)) false false)
    (return)))