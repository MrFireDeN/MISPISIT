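; BP_InteractComponent lets its owner touch, pick up and release objects that implement the CPP_Interactable interface.
; Touch events cache the current Interactable and clear it when that same object is untouched.
; Attach works as a toggle: it detaches any held actor, otherwise snaps the cached Interactable to a mesh socket, keeping world scale.
; Touch, attach and detach each call a matching OnTouch, OnAttach or OnDetach.
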(event Custom|Attach
  (params (SocketName :type Name) (Mesh :type Skeletal%20Mesh%20Component%20Object%20Reference))
  (Utilities|IsValid (Variables|Default|GetAttachedActor)
    (:Is%20Valid
      (CallFunction|Detach))
    (:Is%20Not%20Valid
      (Utilities|IsValid (Variables|Default|GetInteractable)
        (:Is%20Valid
          (bind _output_get (Variables|Default|SetAttachedActor (Variables|Default|GetInteractable)))
          (Transformation|AttachComponentToComponent _output_get Mesh SocketName "SnapToTarget" "SnapToTarget" "KeepWorld" true)
          (Class|InteractableHelper|CallonAttach (Variables|Default|GetAttachedActor)))))))

(event Custom|OnTouch
  (params (Interactable :type Actor%20Object%20Reference))
  (if (Utilities|DoesObjectImplementInterface Interactable "/Script/MISPISIT.CPP_Interactable")
    (bind _output_get (Variables|Default|SetInteractable Interactable))
    (Class|InteractableHelper|CallonTouch _output_get)))

(event Custom|OnUntouch
  (params (Interactable :type Actor%20Object%20Reference))
  (if (== Interactable (Variables|Default|GetInteractable))
    (Variables|Default|SetInteractable 0)))

(event Custom|Detach
  (Transformation|DetachFromActor (Variables|Default|GetAttachedActor) "KeepWorld" "KeepWorld" "KeepWorld")
  (Class|InteractableHelper|CallonDetach (Variables|Default|GetAttachedActor))
  (Variables|Default|SetAttachedActor 0))