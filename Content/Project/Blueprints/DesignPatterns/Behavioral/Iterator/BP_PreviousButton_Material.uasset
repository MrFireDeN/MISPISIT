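; A pressable button Blueprint in an Iterator design pattern sample that steps a slide show back to its previous material.
; On Press, after the parent call, it asks the referenced SlideShowSample's MaterialIterator whether a previous item exists.
; If so, it casts that item to a Material and applies it to the sample mesh's first slot; otherwise it prints a placeholder string.
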(event EventBeginPlay
  (|CallParentFunction) ; This node is disabled and will not be called.\nDrag off pins to build functionality.
)

(event Collision|EventActorBeginOverlap
  (params (OtherActor :type Actor%20Object%20Reference))
  (|CallParentFunction OtherActor) ; This node is disabled and will not be called.\nDrag off pins to build functionality.
)

(event EventTick
  (params (DeltaSeconds :type Float%20%28single-precision%29))
  (|CallParentFunction DeltaSeconds) ; This node is disabled and will not be called.\nDrag off pins to build functionality.
)

(event EventPress
  (bind _slideshowsample (Variables|Default|GetSlideShowSample))
  (bind _materialiterator (Variables|/Game/Project/Blueprints/DesignPatterns/Behavioral/Iterator/BP_SlideShowSample.BP_SlideShowSample_C|GetMaterialIterator _slideshowsample))
  (|CallParentFunction)
  (Utilities|IsValid (Variables|Default|GetSlideShowSample)
    (:Is%20Valid
      (bind _returnvalue (Class|MIAssetIterator|HasPrevious _materialiterator))
      (if _returnvalue
        (bind _returnvalue_2 (Class|MIAssetIterator|GetPrevious _materialiterator))
        (bind _asmaterial (Utilities|Casting|CastToMaterial _returnvalue_2))
        (Rendering|Material|SetMaterial (Variables|/Game/Project/Blueprints/DesignPatterns/Behavioral/Iterator/BP_SlideShowSample.BP_SlideShowSample_C|GetMesh (Variables|Default|GetSlideShowSample)) 0 _asmaterial)
        (else
          (Development|PrintString "Hello"))))))

(fn ConstructionScript
  (|CallParentFunction))