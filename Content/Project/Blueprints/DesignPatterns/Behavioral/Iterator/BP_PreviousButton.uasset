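; BP_PreviousButton is the button that steps a slide show sample back to its previous static mesh, as part of an Iterator design pattern example.
; On Press it runs the parent logic, then asks the referenced SlideShowSample's Iterator whether a previous item exists.
; If one does, it casts that item to a StaticMesh and sets it on the sample's Mesh; otherwise it prints a placeholder string.
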(event EventBeginPlay
  (|CallParentFunction) ; This node is disabled and will not be called.\nDrag off pins to build functionality.
)

(event Collision|EventActorBeginOverlap
  (params (OtherActor :type Actor%20Object%20Reference))
  (|CallParentFunction OtherActor) ; This node is disabled and will not be called.\nDrag off pins to build functionality.
)

(event EventTick
  (params (DeltaSeconds :type Float%20%28single-precision%29))
  (|CallParentFunction DeltaSeconds) ; This node is disabled and will not be called.\nDrag off pins to build functionality.
)

(event EventPress
  (bind _slideshowsample (Variables|Default|GetSlideShowSample))
  (bind _iterator (Variables|/Game/Project/Blueprints/DesignPatterns/Behavioral/Iterator/BP_SlideShowSample.BP_SlideShowSample_C|GetIterator _slideshowsample))
  (|CallParentFunction)
  (Utilities|IsValid (Variables|Default|GetSlideShowSample)
    (:Is%20Valid
      (bind _returnvalue (Class|MIAssetIterator|HasPrevious _iterator))
      (if _returnvalue
        (bind _returnvalue_2 (Class|MIAssetIterator|GetPrevious _iterator))
        (bind _asstatic_mesh (Utilities|Casting|CastToStaticMesh _returnvalue_2))
        (Components|StaticMesh|SetStaticMesh (Variables|/Game/Project/Blueprints/DesignPatterns/Behavioral/Iterator/BP_SlideShowSample.BP_SlideShowSample_C|GetMesh (Variables|Default|GetSlideShowSample)) _asstatic_mesh)
        (else
          (Development|PrintString "Hello"))))))

(fn ConstructionScript
  (|CallParentFunction))