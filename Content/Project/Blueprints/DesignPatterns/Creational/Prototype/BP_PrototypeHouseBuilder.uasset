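; Prototype design pattern demo that assembles a small house by cloning registered building pieces.
; On BeginPlay it spawns a C++ prototype registry, then spawns and styles wall variants, a door, a window and a roof as named prototypes.
; CreateHouse, guarded by DoOnce, requests copies from the registry by name and teleports them to hardcoded world transforms.
; It finishes the house by spawning a point light inside.
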(event Custom|CreateHouse
  (Utilities|FlowControl|DoOnce false
    (:Completed
      (bind _returnvalue (Class|CPPPrototypeRegistry|Create (Variables|Default|GetPrototypeRegisty) "BrickWallForWindow"))
      (Transformation|SetActorTransform _returnvalue (Math|Transform|MakeTransform "2400.000000,2600.000000,2000.000000" "0.000000,180.000000,0.000000" "1.000000,1.000000,1.000000") false true)
      (bind _returnvalue_2 (Class|CPPPrototypeRegistry|Create (Variables|Default|GetPrototypeRegisty) "BrickWallForDoor"))
      (Transformation|SetActorTransform _returnvalue_2 (Math|Transform|MakeTransform "2300.000000,2600.000000,2000.000000" "0.000000,180.000000,0.000000" "1.000000,1.000000,1.000000") false true)
      (bind _returnvalue_3 (Class|CPPPrototypeRegistry|Create (Variables|Default|GetPrototypeRegisty) "ModernDoor"))
      (Transformation|SetActorLocationAndRotation _returnvalue_3 "2300.000000,2600.000000,2000.000000" "0.000000,180.000000,0.000000" false true)
      (bind _returnvalue_4 (Class|CPPPrototypeRegistry|Create (Variables|Default|GetPrototypeRegisty) "BrickWallCorner"))
      (Transformation|SetActorLocationAndRotation _returnvalue_4 "2100.000000,2600.000000,2000.000000" "0.000000,90.000000,0.000000" false true)
      (bind _returnvalue_5 (Class|CPPPrototypeRegistry|Create (Variables|Default|GetPrototypeRegisty) "BrickWall"))
      (Transformation|SetActorLocationAndRotation _returnvalue_5 "2100.000000,2700.000000,2000.000000" "0.000000,90.000000,0.000000" false true)
      (bind _returnvalue_6 (Class|CPPPrototypeRegistry|Create (Variables|Default|GetPrototypeRegisty) "BrickWallCorner"))
      (Transformation|SetActorLocationAndRotation _returnvalue_6 "2100.000000,2900.000000,2000.000000" "0, 0, 0" false true)
      (bind _returnvalue_7 (Class|CPPPrototypeRegistry|Create (Variables|Default|GetPrototypeRegisty) "BrickWall"))
      (Transformation|SetActorLocationAndRotation _returnvalue_7 "2200.000000,2900.000000,2000.000000" "0, 0, 0" false true)
      (bind _returnvalue_8 (Class|CPPPrototypeRegistry|Create (Variables|Default|GetPrototypeRegisty) "BrickWall"))
      (Transformation|SetActorLocationAndRotation _returnvalue_8 "2300.000000,2900.000000,2000.000000" "0, 0, 0" false true)
      (bind _returnvalue_9 (Class|CPPPrototypeRegistry|Create (Variables|Default|GetPrototypeRegisty) "BrickWallCorner"))
      (Transformation|SetActorLocationAndRotation _returnvalue_9 "2500.000000,2900.000000,2000.000000" "0.000000,270.000000,0.000000" false true)
      (bind _returnvalue_10 (Class|CPPPrototypeRegistry|Create (Variables|Default|GetPrototypeRegisty) "BrickWall"))
      (Transformation|SetActorLocationAndRotation _returnvalue_10 "2500.000000,2800.000000,2000.000000" "0.000000,270.000000,0.000000" false true)
      (bind _returnvalue_11 (Class|CPPPrototypeRegistry|Create (Variables|Default|GetPrototypeRegisty) "BrickWallCorner"))
      (Transformation|SetActorLocationAndRotation _returnvalue_11 "2500.000000,2600.000000,2000.000000" "0.000000,180.000000,0.000000" false true)
      (bind _returnvalue_12 (Class|CPPPrototypeRegistry|Create (Variables|Default|GetPrototypeRegisty) "MedievalWindow"))
      (Transformation|SetActorLocationAndRotation _returnvalue_12 "2400.000000,2600.000000,2000.000000" "0.000000,180.000000,0.000000" false true)
      (bind _returnvalue_13 (Class|CPPPrototypeRegistry|Create (Variables|Default|GetPrototypeRegisty) "StoneRoof"))
      (Transformation|SetActorLocationAndRotation _returnvalue_13 "2500.000000,2600.000000,2300.000000" "0.000000,180.000000,0.000000" false true)
      (Game|SpawnActorfromClass "/Script/Engine.PointLight" (Math|Transform|MakeTransform "2300.000000,2800.000000,2200.000000" "0, 0, 0" "1.000000,1.000000,1.000000") "Undefined" "MultiplyWithRoot" 0 0))))

(event EventBeginPlay
  (bind _returnvalue (Game|SpawnActorfromClass "/Script/MISPISIT.CPP_PrototypeRegistry" (Transformation|GetActorTransform) "Undefined" "MultiplyWithRoot" 0 0))
  (Variables|Default|SetPrototypeRegisty _returnvalue)
  ;[1 1 1] BrickWall
  (bind _returnvalue_2 (Game|SpawnActorfromClass "/Script/MISPISIT.CPP_WallPrototype" (Math|Transform|MakeTransform "2700.000000,2000.000000,2000.000000" "0.000000,90.000000,0.000000" "1.000000,1.000000,1.000000") "Undefined" "MultiplyWithRoot" 0 "Default" 0))
  (Class|CPPPrototype|SetStyle _returnvalue_2 "Brick")
  (Class|CPPPrototypeRegistry|Add (Variables|Default|GetPrototypeRegisty) _returnvalue_2 "BrickWall")
  ;[1 1 1] BrickWallCorner
  (bind _returnvalue_3 (Game|SpawnActorfromClass "/Script/MISPISIT.CPP_WallPrototype" (Math|Transform|MakeTransform "2800.000000,2100.000000,2000.000000" "0.000000,180.000000,0.000000" "1.000000,1.000000,1.000000") "Undefined" "MultiplyWithRoot" 0 "Corner" 0))
  (Class|CPPPrototype|SetStyle _returnvalue_3 "Brick")
  (Class|CPPPrototypeRegistry|Add (Variables|Default|GetPrototypeRegisty) _returnvalue_3 "BrickWallCorner")
  ;[1 1 1] BrickWallForWindow
  (bind _returnvalue_4 (Game|SpawnActorfromClass "/Script/MISPISIT.CPP_WallPrototype" (Math|Transform|MakeTransform "2700.000000,2200.000000,2000.000000" "0.000000,90.000000,0.000000" "1.000000,1.000000,1.000000") "Undefined" "MultiplyWithRoot" 0 "ForWindow" 0))
  (Class|CPPPrototype|SetStyle _returnvalue_4 "Brick")
  (Class|CPPPrototypeRegistry|Add (Variables|Default|GetPrototypeRegisty) _returnvalue_4 "BrickWallForWindow")
  ;[1 1 1] BrickWallForDoor
  (bind _returnvalue_5 (Game|SpawnActorfromClass "/Script/MISPISIT.CPP_WallPrototype" (Math|Transform|MakeTransform "2700.000000,2300.000000,2000.000000" "0.000000,90.000000,0.000000" "1.000000,1.000000,1.000000") "Undefined" "MultiplyWithRoot" 0 "UpDoor" 0))
  (Class|CPPPrototype|SetStyle _returnvalue_5 "Brick")
  (Class|CPPPrototypeRegistry|Add (Variables|Default|GetPrototypeRegisty) _returnvalue_5 "BrickWallForDoor")
  ;[1 1 1] ModernDoor
  (bind _returnvalue_6 (Game|SpawnActorfromClass "/Script/MISPISIT.CPP_DoorPrototype" (Math|Transform|MakeTransform "2700.000000,2400.000000,2000.000000" "0.000000,90.000000,0.000000" "1.000000,1.000000,1.000000") "Undefined" "MultiplyWithRoot" 0 0))
  (Class|CPPPrototype|SetStyle _returnvalue_6 "Modern")
  (Class|CPPPrototypeRegistry|Add (Variables|Default|GetPrototypeRegisty) _returnvalue_6 "ModernDoor")
  ;[1 1 1] MedievalWindow
  (bind _returnvalue_7 (Game|SpawnActorfromClass "/Script/MISPISIT.CPP_WindowPrototype" (Math|Transform|MakeTransform "2700.000000,2500.000000,2000.000000" "0.000000,90.000000,0.000000" "1.000000,1.000000,1.000000") "Undefined" "MultiplyWithRoot" 0 0))
  (Class|CPPPrototype|SetStyle _returnvalue_7 "Medieval")
  (Class|CPPPrototypeRegistry|Add (Variables|Default|GetPrototypeRegisty) _returnvalue_7 "MedievalWindow")
  ;[1 1 1] StoneRoof
  (bind _returnvalue_8 (Game|SpawnActorfromClass "/Script/MISPISIT.CPP_RoofPrototype" (Math|Transform|MakeTransform "2700.000000,2600.000000,2000.000000" "0.000000,90.000000,0.000000" "4.000000,3.000000,3.000000") "Undefined" "MultiplyWithRoot" 0 0))
  (Class|CPPPrototype|SetStyle _returnvalue_8 "Stone")
  (Class|CPPPrototypeRegistry|Add (Variables|Default|GetPrototypeRegisty) _returnvalue_8 "StoneRoof"))

(event Collision|EventActorBeginOverlap
  (params (OtherActor :type Actor%20Object%20Reference)))

(event EventTick
  (params (DeltaSeconds :type Float%20%28single-precision%29)))

(fn ConstructionScript)