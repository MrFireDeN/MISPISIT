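; BP_PrototypeButton is a gameplay button that triggers prototype house creation when pressed.
; On BeginPlay it spawns a BP_PrototypeHouseBuilder at its own transform and keeps a reference to it.
; Its Press override runs the parent behavior, then calls CreateHouse on that builder.
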(event EventBeginPlay
  (|CallParentFunction)
  (bind _returnvalue (Game|SpawnActorfromClass "/Game/Project/Blueprints/DesignPatterns/Creational/Prototype/BP_PrototypeHouseBuilder.BP_PrototypeHouseBuilder_C" (Transformation|GetActorTransform) "Undefined" "MultiplyWithRoot" 0 0))
  (Variables|Default|SetHouseBuilder _returnvalue))

(event Collision|EventActorBeginOverlap
  (params (OtherActor :type Actor%20Object%20Reference))
  (|CallParentFunction OtherActor) ; This node is disabled and will not be called.\nDrag off pins to build functionality.
)

(event EventTick
  (params (DeltaSeconds :type Float%20%28single-precision%29))
  (|CallParentFunction DeltaSeconds) ; This node is disabled and will not be called.\nDrag off pins to build functionality.
)

(event EventPress
  (|CallParentFunction)
  (Default|CreateHouse (Variables|Default|GetHouseBuilder)))

(fn ConstructionScript
  (|CallParentFunction))