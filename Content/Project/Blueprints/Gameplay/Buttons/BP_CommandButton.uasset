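; Button Blueprint that, when pressed by a player character, orders a target AI to move to it and look at it.
; On BeginPlay it caches the Target's MIAIController_Command.
; Press runs the parent logic, then for overlapping MIPlayerCharacters creates move-to and look-at command objects.
; It uses the Command pattern: each object is initialized with the controller as receiver and passed to ExecuteCommand.
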(event Custom|Move%20To%20Button
  (bind _returnvalue (Game|ConstructObjectfromClass "/Script/MISPISIT.MIMoveToCommand"))
  (Class|MIMovetoCommand|Initialize _returnvalue (Variables|Default|GetTargetController) (Transformation|GetActorLocation))
  (Class|MIAIControllerCommand|ExecuteCommand (Variables|Default|GetTargetController) _returnvalue))

(event Custom|Look%20At%20Button
  (bind _returnvalue (Game|ConstructObjectfromClass "/Script/MISPISIT.MILookAtCommand"))
  (Class|MILookatCommand|Initialize _returnvalue (Variables|Default|GetTargetController) self)
  (Class|MIAIControllerCommand|ExecuteCommand (Variables|Default|GetTargetController) _returnvalue))

(event EventPress
  (|CallParentFunction)
  (for _array_element (Variables|Default|GetOverlapActors)
    (Utilities|Casting|CastToMIPlayerCharacter _array_element)
    (CallFunction|MovetoButton)
    (CallFunction|LookatButton)))

(event EventBeginPlay
  (bind _target (Variables|Default|GetTarget))
  (|CallParentFunction)
  (Utilities|IsValid _target
    (:Is%20Valid
      (bind _asmiaicontroller_command (Utilities|Casting|CastToMIAIController_Command (Pawn|GetController _target)))
      (Variables|Default|SetTargetController _asmiaicontroller_command))))

(fn ConstructionScript
  (|CallParentFunction))