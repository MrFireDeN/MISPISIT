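; BP_Builder is a pressable button that demonstrates the Builder pattern by spawning weapon variants.
; On BeginPlay it spawns a C++ weapon director and six weapon-type builders, stored as interfaces.
; Each press hands every builder to the director, which creates empty, standard and full weapons.
; The results are placed at hardcoded world locations, offset along X by builder index and variant.
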(event EventBeginPlay
  (|CallParentFunction)
  (bind _returnvalue (Game|SpawnActorfromClass "/Script/MISPISIT.CPP_WeaponDirector" (Math|Transform|MakeTransform "0, 0, 0" "0, 0, 0" "1.000000,1.000000,1.000000") "Undefined" "MultiplyWithRoot" 0 0))
  (Variables|Default|SetWeaponDirector _returnvalue)
  (bind _returnvalue_2 (Game|SpawnActorfromClass "/Script/MISPISIT.CPP_PistolBuilder" (Math|Transform|MakeTransform "0, 0, 0" "0, 0, 0" "1.000000,1.000000,1.000000") "Undefined" "MultiplyWithRoot" 0 0))
  (Utilities|Array|Add (Variables|Default|GetBuilderInterfaces) _returnvalue_2)
  (bind _returnvalue_3 (Game|SpawnActorfromClass "/Script/MISPISIT.CPP_SniperRifleBuilder" (Math|Transform|MakeTransform "0, 0, 0" "0, 0, 0" "1.000000,1.000000,1.000000") "Undefined" "MultiplyWithRoot" 0 0))
  (Utilities|Array|Add (Variables|Default|GetBuilderInterfaces) _returnvalue_3)
  (bind _returnvalue_4 (Game|SpawnActorfromClass "/Script/MISPISIT.CPP_TacticalRifleBuilder" (Math|Transform|MakeTransform "0, 0, 0" "0, 0, 0" "1.000000,1.000000,1.000000") "Undefined" "MultiplyWithRoot" 0 0))
  (Utilities|Array|Add (Variables|Default|GetBuilderInterfaces) _returnvalue_4)
  (bind _returnvalue_5 (Game|SpawnActorfromClass "/Script/MISPISIT.CPP_AssaultRifleBuilder" (Math|Transform|MakeTransform "0, 0, 0" "0, 0, 0" "1.000000,1.000000,1.000000") "Undefined" "MultiplyWithRoot" 0 0))
  (Utilities|Array|Add (Variables|Default|GetBuilderInterfaces) _returnvalue_5)
  (bind _returnvalue_6 (Game|SpawnActorfromClass "/Script/MISPISIT.CPP_MachineGunBuilder" (Math|Transform|MakeTransform "0, 0, 0" "0, 0, 0" "1.000000,1.000000,1.000000") "Undefined" "MultiplyWithRoot" 0 0))
  (Utilities|Array|Add (Variables|Default|GetBuilderInterfaces) _returnvalue_6)
  (bind _returnvalue_7 (Game|SpawnActorfromClass "/Script/MISPISIT.CPP_SMGBuilder" (Math|Transform|MakeTransform "0, 0, 0" "0, 0, 0" "1.000000,1.000000,1.000000") "Undefined" "MultiplyWithRoot" 0 0))
  (Utilities|Array|Add (Variables|Default|GetBuilderInterfaces) _returnvalue_7))

(event EventPress
  (|CallParentFunction)
  (for (_array_element _array_index) (Variables|Default|GetBuilderInterfaces)
    (Class|CPPWeaponDirector|SetBuilder (Variables|Default|GetWeaponDirector) _array_element)
    (Utilities|FlowControl|Sequence
      (:then_0
        (bind _returnvalue (Class|CPPWeaponDirector|CreateEmptyWeapon (Variables|Default|GetWeaponDirector)))
        (Transformation|SetActorLocation _returnvalue (+ (Math|Vector|MakeVector (* _array_index 100) 0.0 0.0) "2000.000000,4600.000000,2100.000000") false false))
      (:then_1
        (bind _returnvalue_2 (Class|CPPWeaponDirector|CreateStandardWeapon (Variables|Default|GetWeaponDirector)))
        (Transformation|SetActorLocation _returnvalue_2 (+ (Math|Vector|MakeVector (* _array_index 100) 0.0 0.0) "2030.000000,4600.000000,2100.000000") false false))
      (:then_2
        (bind _returnvalue_3 (Class|CPPWeaponDirector|CreateFullWeapon (Variables|Default|GetWeaponDirector)))
        (Transformation|SetActorLocation _returnvalue_3 (+ (Math|Vector|MakeVector (* _array_index 100) 0.0 0.0) "2060.000000,4600.000000,2100.000000") false false)))))

(fn ConstructionScript
  (|CallParentFunction))