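; BP_FactoryButton is a button that updates the house through a building factory when pressed.
; On begin play it constructs an object from its configured factory class and caches the game state as BP_MIGameState.
; A press runs CreateHouse, which passes that factory to UpdateHouse on the game state's HouseBilder, so each button's factory class determines what the builder receives.
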(event Custom|CreateHouse
  (Default|UpdateHouse (Variables|/Game/Project/Blueprints/Core/BP_MIGameState.BP_MIGameState_C|GetHouseBilder (Variables|Default|GetAs%20BP%20Game%20State)) (Variables|Default|GetBuildingFactory)))

(event EventBeginPlay
  (|CallParentFunction)
  (bind _returnvalue (Game|ConstructObjectfromClass (Variables|Default|GetCurrentBuildingFactoryClass)))
  (Variables|Default|SetBuildingFactory _returnvalue)
  (Variables|Default|SetAs%20BP%20Game%20State (.AsBP%20MIGame%20State (Utilities|Casting|CastToBP_MIGameState (Game|GetGameState)))))

(event EventPress
  (|CallParentFunction)
  (CallFunction|CreateHouse))

(fn ConstructionScript
  (|CallParentFunction))