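; BP_Button is a pressure button that tracks overlapping actors, pressing on the first arrival and unpressing when the last leaves.
; Press lowers the button mesh and, only once, asks a C++ medieval building factory, constructed at BeginPlay, to create a door, then prints a debug string.
; Unpress sets the mesh to the same lowered position, so it does not visually rise.
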(event Custom|Press
  (Transformation|SetRelativeLocation (Variables|Default|GetButtonMesh) "0.000000,0.000000,-1.000000" false false)
  (Utilities|FlowControl|DoOnce false
    (:Completed
      (Class|CPPBuildingFactory|CreateDoor (Variables|Default|GetBuildingFactory) 1.0 2.0)
      (Development|PrintString "Hello"))))

(event Custom|Unpress
  (Transformation|SetRelativeLocation (Variables|Default|GetButtonMesh) "0.000000,0.000000,-1.000000" false false))

(event EventBeginPlay
  (bind _returnvalue (Game|ConstructObjectfromClass "/Script/MISPISIT.CPP_MedievalBuildingFactory"))
  (Variables|Default|SetBuildingFactory _returnvalue))

(event Collision|EventActorBeginOverlap
  (params (OtherActor :type Actor%20Object%20Reference))
  (Utilities|FlowControl|Sequence
    (:then_0
      (if (Utilities|Array|IsEmpty (Variables|Default|GetOverlapActors))
        (CallFunction|Press)))
    (:then_1
      (Utilities|Array|AddUnique (Variables|Default|GetOverlapActors) OtherActor))))

(event Collision|EventActorEndOverlap
  (params (OtherActor :type Actor%20Object%20Reference))
  (Utilities|Array|RemoveItem (Variables|Default|GetOverlapActors) OtherActor)
  (if (Utilities|Array|IsEmpty (Variables|Default|GetOverlapActors))
    (CallFunction|Unpress)))

(fn ConstructionScript)