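; BP_HouseBuilder assembles a fixed-layout house from pieces spawned by a BuildingFactory.
; UpdateHouse stores the given factory and, if it is valid, destroys the current house and builds a new one, so changing factories rebuilds the same layout.
; Walls, doors, windows and a roof are created at hard-coded transforms and kept in per-type arrays, which DeleteHouse safely destroys and clears.
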(event Custom|ClearBuildingsArray
  (params (BuildingComponents :type Array%20of%20CPP%20Building%20Component%20Object%20References))
  ;[1 1 1] Safe Clear Array
  (for _array_element BuildingComponents
    (Utilities|IsValid _array_element
      (:Is%20Valid
        (Actor|DestroyActor _array_element))))
  (Utilities|Array|Clear BuildingComponents))

(event Custom|DeleteHouse
  ;[1 1 1] Delete House
  (CallFunction|ClearBuildingsArray (Variables|Default|GetDoors))
  (CallFunction|ClearBuildingsArray (Variables|Default|GetWalls))
  (CallFunction|ClearBuildingsArray (Variables|Default|GetWindows))
  (CallFunction|ClearBuildingsArray (Variables|Default|GetRoofs)))

(event Custom|CreateHouse
  ;[1 1 1] Create House
  (CallFunction|CreateWalls)
  (CallFunction|CreateDoors)
  (CallFunction|CreateWindows)
  (CallFunction|CreateRoofs))

(event Custom|UpdateHouse
  (params (BuildingFactory :type CPP%20Building%20Factory%20Object%20Reference))
  ;[1 1 1] Update House
  (bind _output_get (Variables|Default|SetBuildingFactory BuildingFactory))
  (Utilities|IsValid _output_get
    (:Is%20Valid
      (CallFunction|DeleteHouse)
      (CallFunction|CreateHouse))))

(event Custom|CreateWalls
  ;[0 1 0.956] Create Walls
  (bind _returnvalue (Class|CPPBuildingFactory|CreateWall (Variables|Default|GetBuildingFactory) (Math|Transform|MakeTransform "1200.000000,1000.000000,0.000000" "0.000000,90.000000,0.000000" "1.000000,1.000000,1.000000") "Corner"))
  (Utilities|Array|Add (Variables|Default|GetWalls) _returnvalue)
  (bind _returnvalue_2 (Class|CPPBuildingFactory|CreateWall (Variables|Default|GetBuildingFactory) (Math|Transform|MakeTransform "1200.000000,1100.000000,0.000000" "0.000000,90.000000,0.000000" "1.000000,1.000000,1.000000") "UpDoor"))
  (Utilities|Array|Add (Variables|Default|GetWalls) _returnvalue_2)
  (bind _returnvalue_3 (Class|CPPBuildingFactory|CreateWall (Variables|Default|GetBuildingFactory) (Math|Transform|MakeTransform "1200.000000,1200.000000,0.000000" "0.000000,90.000000,0.000000" "1.000000,1.000000,1.000000") "Default"))
  (Utilities|Array|Add (Variables|Default|GetWalls) _returnvalue_3)
  (bind _returnvalue_4 (Class|CPPBuildingFactory|CreateWall (Variables|Default|GetBuildingFactory) (Math|Transform|MakeTransform "1200.000000,1300.000000,0.000000" "0.000000,90.000000,0.000000" "1.000000,1.000000,1.000000") "ForWindow"))
  (Utilities|Array|Add (Variables|Default|GetWalls) _returnvalue_4)
  (bind _returnvalue_5 (Class|CPPBuildingFactory|CreateWall (Variables|Default|GetBuildingFactory) (Math|Transform|MakeTransform "1200.000000,1500.000000,0.000000" "0.000000,0.000000,0.000000" "1.000000,1.000000,1.000000") "Corner"))
  (Utilities|Array|Add (Variables|Default|GetWalls) _returnvalue_5)
  (bind _returnvalue_6 (Class|CPPBuildingFactory|CreateWall (Variables|Default|GetBuildingFactory) (Math|Transform|MakeTransform "1300.000000,1500.000000,0.000000" "0, 0, 0" "1.000000,1.000000,1.000000") "Default"))
  (Utilities|Array|Add (Variables|Default|GetWalls) _returnvalue_6)
  (bind _returnvalue_7 (Class|CPPBuildingFactory|CreateWall (Variables|Default|GetBuildingFactory) (Math|Transform|MakeTransform "1500.000000,1500.000000,0.000000" "0.000000,270.000000,0.000000" "1.000000,1.000000,1.000000") "Corner"))
  (Utilities|Array|Add (Variables|Default|GetWalls) _returnvalue_7)
  (bind _returnvalue_8 (Class|CPPBuildingFactory|CreateWall (Variables|Default|GetBuildingFactory) (Math|Transform|MakeTransform "1500.000000,1400.000000,0.000000" "0.000000,270.000000,0.000000" "1.000000,1.000000,1.000000") "ForWindow"))
  (Utilities|Array|Add (Variables|Default|GetWalls) _returnvalue_8)
  (bind _returnvalue_9 (Class|CPPBuildingFactory|CreateWall (Variables|Default|GetBuildingFactory) (Math|Transform|MakeTransform "1500.000000,1300.000000,0.000000" "0.000000,270.000000,0.000000" "1.000000,1.000000,1.000000") "Default"))
  (Utilities|Array|Add (Variables|Default|GetWalls) _returnvalue_9)
  (bind _returnvalue_10 (Class|CPPBuildingFactory|CreateWall (Variables|Default|GetBuildingFactory) (Math|Transform|MakeTransform "1500.000000,1200.000000,0.000000" "0.000000,270.000000,0.000000" "1.000000,1.000000,1.000000") "ForWindow"))
  (Utilities|Array|Add (Variables|Default|GetWalls) _returnvalue_10)
  (bind _returnvalue_11 (Class|CPPBuildingFactory|CreateWall (Variables|Default|GetBuildingFactory) (Math|Transform|MakeTransform "1500.000000,1000.000000,0.000000" "0.000000,180.000000,0.000000" "1.000000,1.000000,1.000000") "Corner"))
  (Utilities|Array|Add (Variables|Default|GetWalls) _returnvalue_11)
  (bind _returnvalue_12 (Class|CPPBuildingFactory|CreateWall (Variables|Default|GetBuildingFactory) (Math|Transform|MakeTransform "1400.000000,1000.000000,0.000000" "0.000000,180.000000,0.000000" "1.000000,1.000000,1.000000") "Default"))
  (Utilities|Array|Add (Variables|Default|GetWalls) _returnvalue_12))

(event Custom|CreateDoors
  ;[0 1 0.956] Create Doors
  (bind _returnvalue (Class|CPPBuildingFactory|CreateDoor (Variables|Default|GetBuildingFactory) (Math|Transform|MakeTransform "1200.000000,1100.000000,0.000000" "0.000000,90.000000,0.000000" "1.000000,1.000000,1.000000")))
  (Utilities|Array|Add (Variables|Default|GetDoors) _returnvalue))

(event Custom|CreateWindows
  ;[0 1 0.956] Create Windows
  (bind _returnvalue (Class|CPPBuildingFactory|CreateWindow (Variables|Default|GetBuildingFactory) (Math|Transform|MakeTransform "1200.000000,1300.000000,0.000000" "0.000000,90.000000,0.000000" "1.000000,1.000000,1.000000")))
  (Utilities|Array|Add (Variables|Default|GetWindows) _returnvalue)
  (bind _returnvalue_2 (Class|CPPBuildingFactory|CreateWindow (Variables|Default|GetBuildingFactory) (Math|Transform|MakeTransform "1500.000000,1200.000000,0.000000" "0.000000,270.000000,0.000000" "1.000000,1.000000,1.000000")))
  (Utilities|Array|Add (Variables|Default|GetWindows) _returnvalue_2)
  (bind _returnvalue_3 (Class|CPPBuildingFactory|CreateWindow (Variables|Default|GetBuildingFactory) (Math|Transform|MakeTransform "1500.000000,1400.000000,0.000000" "0.000000,270.000000,0.000000" "1.000000,1.000000,1.000000")))
  (Utilities|Array|Add (Variables|Default|GetWindows) _returnvalue_3))

(event Custom|CreateRoofs
  ;[0 1 0.956] Create Roofs
  (bind _returnvalue (Class|CPPBuildingFactory|CreateRoof (Variables|Default|GetBuildingFactory) (Math|Transform|MakeTransform "1200.000000,1000.000000,300.000000" "0.000000,90.000000,0.000000" "5.000000,3.000000,2.000000")))
  (Utilities|Array|Add (Variables|Default|GetRoofs) _returnvalue))

(event EventBeginPlay)

(event Collision|EventActorBeginOverlap
  (params (OtherActor :type Actor%20Object%20Reference)))

(event EventTick
  (params (DeltaSeconds :type Float%20%28single-precision%29)))

(fn ConstructionScript)